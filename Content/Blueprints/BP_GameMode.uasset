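; Game mode Blueprint that runs a minutes-and-seconds countdown and pauses the game when it runs out of minutes.
; Tick feeds a one-second Delay, which throttles the countdown to roughly one step per second.
; When Seconds drops below zero it wraps and decrements Minutes, pausing as soon as Minutes reaches zero, with Seconds just reset to 59.
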(event EventBeginPlay)

(event EventTick
  (params (DeltaSeconds :type Float%20%28single-precision%29))
  (Utilities|FlowControl|Delay 1.0)
  (bind _output_get (Variables|Default|Setseconds (- (Variables|Default|Getseconds) 1)))
  (if (< _output_get 0)
    (Variables|Default|Setseconds 59)
    (Variables|Default|Setminutes (- (Variables|Default|Getminutes) 1))
    (if (<= (Variables|Default|Getminutes) 0)
      (Game|SetGamePaused true))))

(fn ConstructionScript)